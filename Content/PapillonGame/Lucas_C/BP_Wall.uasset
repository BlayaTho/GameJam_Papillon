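; BP_Wall is a wall actor that fades by animating the WallFade scalar on its SWallA component's material.
; BeginPlay creates and stores a dynamic material instance from the first material slot.
; Fadeout plays a timeline that lerps WallFade from 1 toward 0, and FadeIn reverses it.
; LightON drives the same parameter with the same lerp through a separate timeline, with no reverse event.
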(event `self.ReceiveBeginPlay`
  (bind _returnvalue (`PrimitiveComponent.CreateDynamicMaterialInstance` (`self.S_Wall_A`) 0 (`PrimitiveComponent.GetMaterial` (`self.S_Wall_A`) 0) "None"))
  (set `self.Dyna` _returnvalue))

(event `Fadeout`
  (bind (_direction _newtrack_0) (`Timeline|Timeline` :!label _label)
    (:`Update`
      (`MaterialInstanceDynamic.SetScalarParameterValue` (`self.Dyna`) "WallFade" (`KismetMathLibrary.Lerp` 1.0 0.0 _newtrack_0)))))

(event `FadeIn`
  (goto _label :!via `Reverse`))

(event `LightON`
  (bind (_direction _newtrack_0) (`Timeline|Timeline_0`)
    (:`Update`
      (`MaterialInstanceDynamic.SetScalarParameterValue` (`self.Dyna`) "WallFade" (`KismetMathLibrary.Lerp` 1.0 0.0 _newtrack_0)))))

(fn `UserConstructionScript`)