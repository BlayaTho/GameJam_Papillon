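; BP_Caisse is a crate that the player character can grab and that respawns at a random spot.
; On BeginPlay it caches the third-person character, then moves its Cube to the location of a random child of BASE; ResetCaisse repeats that move.
; The random index is drawn below LastIndex, so the last child is never picked.
; The Interaction event delegates to the character's Grab.
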(event `ResetCaisse`
  (bind _children (`SceneComponent.GetChildrenComponents` (`self.BASE`) false))
  (`SceneComponent.K2_SetWorldLocation` (`self.Cube`) (`SceneComponent.K2_GetComponentLocation` (`|GetArrayItem` _children (`KismetMathLibrary.RandomInteger` (`KismetArrayLibrary.Array_LastIndex` _children)))) false false :!label _label))

(event `self.ReceiveBeginPlay`
  (bind _asbp_third_person_character (cast `/Game/PapillonGame/Thomas_B/ThirdPerson/Blueprints/BP_ThirdPersonCharacter` (`GameplayStatics.GetPlayerCharacter` 0)))
  (set `self.As BP Third Person Character` _asbp_third_person_character)
  (goto _label))

(event `/Game/PapillonGame/Thomas_B/Interface/BPI_Interaction.Interaction`
  (`/Game/PapillonGame/Thomas_B/ThirdPerson/Blueprints/BP_ThirdPersonCharacter.Grab` (`self.As BP Third Person Character`)))

(fn `UserConstructionScript`)