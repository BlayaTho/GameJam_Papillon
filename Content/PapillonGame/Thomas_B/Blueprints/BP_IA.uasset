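; Ghost actor (BP_IA) that replays the player's recorded path and destroys any player character it touches.
; While CanCount is set, Tick records player location and rotation into parallel arrays until FinCompte switches to playback.
; With CanFollow and Follow set, Tick moves the capsule one sample per frame, looping.
; FinNiveauReset repositions it and resumes after a delay; box overlap also attempts a ScoreP penalty after the destroy.
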(event `self.ReceiveBeginPlay`
  ;[0.1615 0.1615 0.1615] BEGIN PLAY
  (bind _asbp_third_person_character (cast `/Game/PapillonGame/Thomas_B/ThirdPerson/Blueprints/BP_ThirdPersonCharacter` (`GameplayStatics.GetPlayerCharacter` 0)))
  (set `self.As BP Third Person Character` _asbp_third_person_character))

(event `FinCompte`
  ;[0.2031 0.2031 0.2031] Fin Compte
  (set `self.CanCount?` false)
  (set `self.CanFollow?` true))

(event `self.ReceiveTick`
  (params (DeltaSeconds :type "Float (single-precision)"))
  (bind _index (`self.Index`))
  (bind _as_bp_third_person_character (`self.As BP Third Person Character`))
  (`|ExecutionSequence`
    (:`then_0`
      ;[1 1 1] Compte les positions du joueur
      (if (`self.CanCount?`)
        (`/Engine/EditorBlueprintResources/StandardMacros.IsValid` _as_bp_third_person_character
          (:`Is Valid`
            (`KismetArrayLibrary.Array_Add` (`self.PositionFantome`) (`self.K2_GetActorLocation` _as_bp_third_person_character))
            (bind _returnvalue (`KismetArrayLibrary.Array_Add` (`self.RotationFantome`) (`self.K2_GetActorRotation` _as_bp_third_person_character)))
            (set `self.NumberOfIndex` _returnvalue)))))
    (:`then_1`
      ;[1 1 1] Follow player
      (if (and (`self.CanFollow?`) (`self.Follow?`))
        (bind _output_get (set `self.Index` (`KismetMathLibrary.Clamp` (+ (`self.Index`) 1) 0 (`self.NumberOfIndex`))))
        (if (== _output_get (`self.NumberOfIndex`))
          (set `self.Index` 0))
        (`SceneComponent.K2_SetRelativeLocationAndRotation` (`self.CapsuleComponent`) (`|GetArrayItem` (`self.PositionFantome`) _index) (`|GetArrayItem` (`self.RotationFantome`) _index) false false)))))

(event `FinNiveauReset`
  ;[1 1 1] EVENT FIN SECTION
  (set `self.Follow?` false)
  (`SceneComponent.K2_SetRelativeLocationAndRotation` :`self` (`self.CapsuleComponent`) :`NewLocation` (70.0 127.0 102.0))
  (if (`self.CanFollow?`)
    (set `self.Index` 0)
    (`KismetSystemLibrary.Delay` 3.0)
    (set `self.Follow?` true)))

(event `self.Box.OnComponentBeginOverlap`
  (params (OverlappedComponent :type "PrimitiveComponent Object Reference") (OtherActor :type "Actor Object Reference") (OtherComp :type "PrimitiveComponent Object Reference") (OtherBodyIndex :type Integer) (bFromSweep :type Boolean) (SweepResult :type "HitResult Structure (by ref)"))
  ;[1 1 1] Event Kill Player
  (bind _asbp_third_person_character (cast `/Game/PapillonGame/Thomas_B/ThirdPerson/Blueprints/BP_ThirdPersonCharacter` OtherActor))
  (`self.K2_DestroyActor` _asbp_third_person_character)
  (bind _asbp_third_person_character_2 (cast `/Game/PapillonGame/Thomas_B/ThirdPerson/Blueprints/BP_ThirdPersonCharacter` (`GameplayStatics.GetPlayerCharacter` 0)))
  (set `/Game/PapillonGame/Thomas_B/ThirdPerson/Blueprints/BP_ThirdPersonCharacter.ScoreP` (+ (`/Game/PapillonGame/Thomas_B/ThirdPerson/Blueprints/BP_ThirdPersonCharacter.ScoreP` _asbp_third_person_character_2) -100) _asbp_third_person_character_2))

(fn `UserConstructionScript`)