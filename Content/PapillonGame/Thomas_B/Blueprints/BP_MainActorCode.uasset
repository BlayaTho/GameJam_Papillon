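; BP_MainActorCode runs a four-color code puzzle driven by the level's BP_PressurePlate actors.
; On BeginPlay it shuffles a non-repeating code, shows it as materials on four cubes, and assigns each plate a different color.
; AddInput checks entries against the code as they arrive, resetting plates and input on a mismatch.
; A full match also resets, then redistributes plate colors while keeping the same code.
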(event `self.ReceiveBeginPlay`
  (bind _outactors (`GameplayStatics.GetAllActorsOfClass` "/Game/PapillonGame/Thomas_B/Blueprints/BP_PressurePlate.BP_PressurePlate_C"))
  (set `self.EachPressurePlate` _outactors)
  (`self.GenerateCode`))

(event `GenerateCode`
  (`KismetArrayLibrary.Array_Clear` (`self.RdmCode`))
  (set `self.Selector` (`|MakeArray` "NewEnumerator0" "NewEnumerator1" "NewEnumerator2" "NewEnumerator3" :!type "/Game/PapillonGame/Thomas_B/Blueprints/Enum_Color Enum"))
  (for _ (range 4)
    (bind _returnvalue (`KismetArrayLibrary.Array_Add` (`self.RdmCode`) (`KismetArrayLibrary.Array_Random` (`self.Selector`))))
    (`KismetArrayLibrary.Array_RemoveItem` (`self.Selector`) (`|GetArrayItem` (`self.RdmCode`) _returnvalue)))
  (`self.SetVisual`)
  (`self.SelectRdmColorOnEachPressurePlate`))

(event `SetVisual`
  (`self.SetColorOnMat` (`self.Cube1`))
  (`self.SetColorOnMat` (`self.Cube4`) 1)
  (`self.SetColorOnMat` (`self.Cube2`) 2)
  (`self.SetColorOnMat` (`self.Cube3`) 3))

(event `SelectRdmColorOnEachPressurePlate`
  (`KismetArrayLibrary.Array_Clear` (`self.Selector`))
  (set `self.Selector` (`|MakeArray` "NewEnumerator0" "NewEnumerator1" "NewEnumerator2" "NewEnumerator3" :!type "/Game/PapillonGame/Thomas_B/Blueprints/Enum_Color Enum"))
  (for _array_element (`self.EachPressurePlate`)
    (`/Game/PapillonGame/Thomas_B/Blueprints/BP_PressurePlate.SetRdmColor` _array_element (`self.Selector`))
    (`KismetArrayLibrary.Array_RemoveItem` (`self.Selector`) (`/Game/PapillonGame/Thomas_B/Blueprints/BP_PressurePlate.RdmColorToSelect` _array_element))))

(event `AddInput`
  (params (ColorToAdd :type "/Game/PapillonGame/Thomas_B/Blueprints/Enum_Color Enum" :default "NewEnumerator0"))
  (`KismetArrayLibrary.Array_Add` (`self.InputCode`) ColorToAdd)
  (`self.CheckForCode`))

(event `CheckForCode`
  (set `self.CodeIsValid` true)
  (if (`KismetArrayLibrary.Array_Identical` (`self.RdmCode`) (`self.InputCode`))
    (`self.CodeIsNice`)
    (else
      (for (_array_element _array_index) (`self.InputCode`) :!label _label
        (if (not (`|EnumEquality` (`|GetArrayItem` (`self.RdmCode`) _array_index) _array_element))
          (set `self.CodeIsValid` false)
          (`self.BreakCodeChecking`)))
      (if (not (`self.CodeIsValid`))
        (`self.ResetTry`)))))

(event `BreakCodeChecking`
  (goto _label :!via `Break`))

(event `CodeIsNice`
  (`self.ResetTry`)
  (`self.SelectRdmColorOnEachPressurePlate`))

(event `ResetTry`
  (for _array_element (`self.EachPressurePlate`)
    (`/Game/PapillonGame/Thomas_B/Blueprints/BP_PressurePlate.ResetCodeToInput` _array_element))
  (`KismetArrayLibrary.Array_Clear` (`self.InputCode`)))

(fn `SetColorOnMat`
  (params (self2 :type "PrimitiveComponent Object Reference") (`Dimension 1` :type Integer))
  (`PrimitiveComponent.SetMaterial` self2 0 (select `/Game/PapillonGame/Thomas_B/Blueprints/Enum_Color` (`|GetArrayItem` (`self.RdmCode`) `Dimension 1`) :`NewEnumerator0` "/Game/PapillonGame/Thomas_B/Materials/M_MatPlaque_Inst2.M_MatPlaque_Inst2" :`NewEnumerator1` "/Game/PapillonGame/Thomas_B/Materials/M_MatPlaque_Inst1.M_MatPlaque_Inst1" :`NewEnumerator2` "/Game/PapillonGame/Thomas_B/Materials/M_MatPlaque_Inst4.M_MatPlaque_Inst4" :`NewEnumerator3` "/Game/PapillonGame/Thomas_B/Materials/M_MatPlaque_Inst3.M_MatPlaque_Inst3" :!type "MaterialInterface Object Reference")))

(fn `UserConstructionScript`)