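; BP_ObjetRepear is an interactable button object that counts toward level completion and awards score.
; Interaction turns its Sphere green, sets ButtonDone on the Bp_FinNiveau actor found at BeginPlay, and adds 5 to the player character's ScoreP.
; A DoOnce blocks repeat interactions until ResetButton turns the sphere red and re-arms it, without clearing ButtonDone or the score.
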(event `self.ReceiveBeginPlay`
  (bind _returnvalue (`GameplayStatics.GetActorOfClass` "/Game/PapillonGame/Thomas_B/Blueprints/Bp_FinNiveau.Bp_FinNiveau_C"))
  (bind _output_get (set `self.RefFinNiveau` _returnvalue)))

(event `/Game/PapillonGame/Thomas_B/Interface/BPI_Interaction.Interaction`
  (`/Engine/EditorBlueprintResources/StandardMacros.DoOnce` false :!label _label
    (:`Completed`
      (`MeshComponent.SetVectorParameterValueOnMaterials` (`self.Sphere`) "Color" (`self.ColorGreen`))
      (set `/Game/PapillonGame/Thomas_B/Blueprints/Bp_FinNiveau.ButtonDone` true (stale `self.ReceiveBeginPlay` _output_get))
      (bind _asbp_third_person_character (cast `/Game/PapillonGame/Thomas_B/ThirdPerson/Blueprints/BP_ThirdPersonCharacter` (`GameplayStatics.GetPlayerCharacter` 0)))
      (set `/Game/PapillonGame/Thomas_B/ThirdPerson/Blueprints/BP_ThirdPersonCharacter.ScoreP` (+ (`/Game/PapillonGame/Thomas_B/ThirdPerson/Blueprints/BP_ThirdPersonCharacter.ScoreP` _asbp_third_person_character) 5) _asbp_third_person_character))))

(event `ResetButton`
  (`MeshComponent.SetVectorParameterValueOnMaterials` (`self.Sphere`) "Color" (`self.ColorRed`))
  (goto _label :!via `Reset`))

(fn `UserConstructionScript`)