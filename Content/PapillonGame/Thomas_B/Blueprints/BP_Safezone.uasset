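; BP_Safezone is a trigger box that makes the player character safe from death while overlapped.
; It caches the BP_ThirdPersonCharacter on BeginPlay, then clears its CanDie on begin overlap and sets it on end overlap, without checking which actor overlapped.
; End overlap also sets CanCount on every BP_IA that cannot follow.
; Both overlaps print debug text, and an unconnected copy of the BP_IA loop never runs.
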(event `self.ReceiveBeginPlay`
  (bind _asbp_third_person_character (cast `/Game/PapillonGame/Thomas_B/ThirdPerson/Blueprints/BP_ThirdPersonCharacter` (`GameplayStatics.GetPlayerCharacter` 0)))
  (set `self.As BP Third Person Character` _asbp_third_person_character))

(event `self.Box.OnComponentBeginOverlap`
  (params (OverlappedComponent :type "PrimitiveComponent Object Reference") (OtherActor :type "Actor Object Reference") (OtherComp :type "PrimitiveComponent Object Reference") (OtherBodyIndex :type Integer) (bFromSweep :type Boolean) (SweepResult :type "HitResult Structure (by ref)"))
  (set `/Game/PapillonGame/Thomas_B/ThirdPerson/Blueprints/BP_ThirdPersonCharacter.CanDie?` false (`self.As BP Third Person Character`))
  (`KismetSystemLibrary.PrintString` "SAFE" true true (struct :`G` 1.0 :`B` 0.748173 :`A` 1.0)))

(event `self.Box.OnComponentEndOverlap`
  (params (OverlappedComponent :type "PrimitiveComponent Object Reference") (OtherActor :type "Actor Object Reference") (OtherComp :type "PrimitiveComponent Object Reference") (OtherBodyIndex :type Integer))
  (set `/Game/PapillonGame/Thomas_B/ThirdPerson/Blueprints/BP_ThirdPersonCharacter.CanDie?` true (`self.As BP Third Person Character`))
  (`KismetSystemLibrary.PrintString` "NOTSAFE" true true (struct :`R` 1.0 :`G` 0.022275 :`B` 0.854225 :`A` 1.0))
  (bind _outactors (`GameplayStatics.GetAllActorsOfClass` "/Game/PapillonGame/Thomas_B/Blueprints/BP_IA.BP_IA_C"))
  (for _array_element _outactors
    (if (not (`/Game/PapillonGame/Thomas_B/Blueprints/BP_IA.CanFollow?` _array_element))
      (set `/Game/PapillonGame/Thomas_B/Blueprints/BP_IA.CanCount?` true _array_element))))

(fn `UserConstructionScript`)