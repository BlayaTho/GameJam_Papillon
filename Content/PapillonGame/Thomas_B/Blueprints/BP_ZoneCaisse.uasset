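; BP_ZoneCaisse is a trigger zone that validates a crate-placement objective for the level.
; On BeginPlay it caches the level's Bp_FinNiveau actor.
; When a BP_Caisse enters its Box, it sets CaisseDone on that actor and adds points to the player character's ScoreP.
; When a crate leaves, it clears the flag and removes those points, printing a debug message in both cases.
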(event `self.ReceiveBeginPlay`
  (bind _returnvalue (`GameplayStatics.GetActorOfClass` "/Game/PapillonGame/Thomas_B/Blueprints/Bp_FinNiveau.Bp_FinNiveau_C"))
  (set `self.RefFin` _returnvalue))

(event `self.Box.OnComponentBeginOverlap`
  (params (OverlappedComponent :type "PrimitiveComponent Object Reference") (OtherActor :type "Actor Object Reference") (OtherComp :type "PrimitiveComponent Object Reference") (OtherBodyIndex :type Integer) (bFromSweep :type Boolean) (SweepResult :type "HitResult Structure (by ref)"))
  (cast `/Game/PapillonGame/Thomas_B/Blueprints/BP_Caisse` OtherActor)
  (`KismetSystemLibrary.PrintString` "Mission Reussi")
  (set `/Game/PapillonGame/Thomas_B/Blueprints/Bp_FinNiveau.CaisseDone` true (`self.RefFin`))
  (bind _asbp_third_person_character (cast `/Game/PapillonGame/Thomas_B/ThirdPerson/Blueprints/BP_ThirdPersonCharacter` (`GameplayStatics.GetPlayerCharacter` 0)))
  (set `/Game/PapillonGame/Thomas_B/ThirdPerson/Blueprints/BP_ThirdPersonCharacter.ScoreP` (+ (`/Game/PapillonGame/Thomas_B/ThirdPerson/Blueprints/BP_ThirdPersonCharacter.ScoreP` _asbp_third_person_character) 10) _asbp_third_person_character))

(event `self.Box.OnComponentEndOverlap`
  (params (OverlappedComponent :type "PrimitiveComponent Object Reference") (OtherActor :type "Actor Object Reference") (OtherComp :type "PrimitiveComponent Object Reference") (OtherBodyIndex :type Integer))
  (cast `/Game/PapillonGame/Thomas_B/Blueprints/BP_Caisse` OtherActor)
  (`KismetSystemLibrary.PrintString` "Cube sorti")
  (set `/Game/PapillonGame/Thomas_B/Blueprints/Bp_FinNiveau.CaisseDone` false (`self.RefFin`))
  (bind _asbp_third_person_character (cast `/Game/PapillonGame/Thomas_B/ThirdPerson/Blueprints/BP_ThirdPersonCharacter` (`GameplayStatics.GetPlayerCharacter` 0)))
  (set `/Game/PapillonGame/Thomas_B/ThirdPerson/Blueprints/BP_ThirdPersonCharacter.ScoreP` (+ (`/Game/PapillonGame/Thomas_B/ThirdPerson/Blueprints/BP_ThirdPersonCharacter.ScoreP` _asbp_third_person_character) -10) _asbp_third_person_character))

(fn `UserConstructionScript`)