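; End-of-level trigger that runs a repeating level loop and creates the objective, timer and tutorial widgets.
; Plate, button and crate finish events set completion flags and objective checkmarks; entering the box with all three done ends the round.
; Completion teleports the player to respawn, resets every AI, spawns an additional BP_IA, resets puzzles and timer, and awards score.
; A DoOnce, re-armed after a short delay, guards against double triggering.
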(event `self.ReceiveBeginPlay`
  ;[1 1 1] Spawn premiere IA
  (bind _returnvalue (`|SpawnActorFromClass` "/Game/PapillonGame/Thomas_B/Blueprints/BP_IA.BP_IA_C" (`self.GetTransform` (`self.RespawnAIREF`)) "Undefined" "MultiplyWithRoot" null null))
  (set `self.REFIA` _returnvalue)
  (`KismetArrayLibrary.Array_Add` (`self.AI_Array`) _returnvalue)
  (bind _asbp_third_person_character (cast `/Game/PapillonGame/Thomas_B/ThirdPerson/Blueprints/BP_ThirdPersonCharacter` (`GameplayStatics.GetPlayerCharacter` 0)))
  (set `self.As BP Third Person Character` _asbp_third_person_character)
  (bind _returnvalue_2 (`|CreateWidget` "/Game/PapillonGame/Thomas_B/HUD/W_Objectif.W_Objectif_C"))
  (bind _output_get (set `self.W_Objectif` _returnvalue_2))
  (`UserWidget.AddToViewport` _output_get 0)
  (bind _returnvalue_3 (`|CreateWidget` "/Game/PapillonGame/Celyan_F/W_timerC.W_timerC_C"))
  (bind _output_get_2 (set `self.W_Timer` _returnvalue_3))
  (`UserWidget.AddToViewport` _returnvalue_3 0)
  (`UserWidget.AddToViewport` _output_get_2 0)
  (set `/Game/PapillonGame/Celyan_F/W_timerC.TempMax` (`self.TempsMAX`) _output_get_2)
  (`/Game/PapillonGame/Celyan_F/W_timerC.SetTextUIMax` _output_get_2)
  (bind _returnvalue_4 (`|CreateWidget` "/Game/PapillonGame/Thomas_B/HUD/W_Tuto.W_Tuto_C"))
  (`UserWidget.AddToViewport` _returnvalue_4 0))

(event `self.Box.OnComponentBeginOverlap`
  (params (OverlappedComponent :type "PrimitiveComponent Object Reference") (OtherActor :type "Actor Object Reference") (OtherComp :type "PrimitiveComponent Object Reference") (OtherBodyIndex :type Integer) (bFromSweep :type Boolean) (SweepResult :type "HitResult Structure (by ref)"))
  (cast `/Game/PapillonGame/Thomas_B/ThirdPerson/Blueprints/BP_ThirdPersonCharacter` OtherActor)
  (if (and (`self.PlaqueDone`) (`self.ButtonDone`) (`self.CaisseDone`))
    (`/Engine/EditorBlueprintResources/StandardMacros.DoOnce` false :!label _label
      (:`Completed`
        (`/Game/PapillonGame/Thomas_B/Blueprints/BP_IA.FinCompte` (`self.REFIA`))
        (for _array_element (`self.AI_Array`)
          (`/Game/PapillonGame/Thomas_B/Blueprints/BP_IA.FinNiveaureset` _array_element))
        (`self.K2_SetActorLocationAndRotation` :`self` (`self.As BP Third Person Character`) :`NewLocation` (`self.K2_GetActorLocation` (`self.RespawnPlayerREF`)))
        (bind _returnvalue (`|SpawnActorFromClass` "/Game/PapillonGame/Thomas_B/Blueprints/BP_IA.BP_IA_C" (`self.GetTransform` (`self.RespawnAIREF`)) "Undefined" "MultiplyWithRoot" null null))
        (set `self.REFIA` _returnvalue)
        (`KismetArrayLibrary.Array_Add` (`self.AI_Array`) _returnvalue)
        (`/Game/PapillonGame/Thomas_B/Blueprints/BP_ObjetRepear.ResetButton` (`self.REFRepair`))
        (`/Game/PapillonGame/Thomas_B/Blueprints/BP_Caisse.ResetCaisse` (`self.REFCaisse`))
        (`/Game/PapillonGame/Thomas_B/Blueprints/BP_MainActorCode.SelectRdmColorOnEachPressurePlate` (`self.REFPLAQUE`))
        (set `/Game/PapillonGame/Celyan_F/W_timerC.time` 0.0 (`self.W_Timer`))
        (`KismetSystemLibrary.Delay` 0.05)
        (`self.resetDo once`)
        (bind _asbp_third_person_character (cast `/Game/PapillonGame/Thomas_B/ThirdPerson/Blueprints/BP_ThirdPersonCharacter` (`GameplayStatics.GetPlayerCharacter` 0)))
        (set `/Game/PapillonGame/Thomas_B/ThirdPerson/Blueprints/BP_ThirdPersonCharacter.ScoreP` (+ (`/Game/PapillonGame/Thomas_B/ThirdPerson/Blueprints/BP_ThirdPersonCharacter.ScoreP` _asbp_third_person_character) 100) _asbp_third_person_character)))))

(event `resetDo once`
  (bind _w_objectif (`self.W_Objectif`))
  (`Widget.SetRenderOpacity` (`/Game/PapillonGame/Thomas_B/HUD/W_Objectif.FINButton` _w_objectif) 0.0)
  (`Widget.SetRenderOpacity` (`/Game/PapillonGame/Thomas_B/HUD/W_Objectif.FINPlaque` _w_objectif) 0.0)
  (`Widget.SetRenderOpacity` (`/Game/PapillonGame/Thomas_B/HUD/W_Objectif.FINCaisse` _w_objectif) 0.0)
  (set `self.PlaqueDone` false)
  (set `self.ButtonDone` false)
  (set `self.CaisseDone` false)
  (goto _label :!via `Reset`))

(event `PlaqueFinish`
  (set `self.PlaqueDone` true)
  (`Widget.SetRenderOpacity` (`/Game/PapillonGame/Thomas_B/HUD/W_Objectif.FINPlaque` (`self.W_Objectif`)) 1.0))

(event `ButtonFinish`
  (set `self.ButtonDone` true)
  (`Widget.SetRenderOpacity` (`/Game/PapillonGame/Thomas_B/HUD/W_Objectif.FINButton` (`self.W_Objectif`)) 1.0))

(event `CaisseFinish`
  (params (`On?` :type Boolean))
  (bind _fincaisse (`/Game/PapillonGame/Thomas_B/HUD/W_Objectif.FINCaisse` (`self.W_Objectif`)))
  (if `On?`
    (set `self.CaisseDone` true)
    (`Widget.SetRenderOpacity` _fincaisse 1.0)
    (else
      (set `self.CaisseDone` false)
      (`Widget.SetRenderOpacity` _fincaisse 0.0))))

(fn `UserConstructionScript`)