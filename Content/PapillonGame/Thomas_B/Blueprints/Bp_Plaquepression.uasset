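; Colour-sequence pressure plate puzzle that marks PlaqueDone on the level's Bp_FinNiveau when the player steps on plates in the correct order.
; ResetPlaque spawns a row of coloured meshes from a randomly picked layout, each with an overlap box tagged by its colour letter.
; Character overlaps feed that letter to AddCode, which checks it against CorrectCode one step at a time and clears the input on a mistake.
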(event `self.ReceiveBeginPlay`
  (bind _returnvalue (`GameplayStatics.GetActorOfClass` "/Game/PapillonGame/Thomas_B/Blueprints/Bp_FinNiveau.Bp_FinNiveau_C"))
  (set `self.RefFinNiveau` _returnvalue))

(event `ResetPlaque`
  (set `self.RandomCode` (`|GetArrayItem` (`self.RandomColor`) (`KismetMathLibrary.RandomInteger` 12)))
  (for _index (range (`KismetStringLibrary.Len` (`self.CorrectCode`)))
    (bind _returnvalue (`AddComponent|NODE_AddStaticMeshComponent-2` :`RelativeTransform` (`KismetMathLibrary.MakeTransform` (`KismetMathLibrary.MakeVector` (* _index (`self.Spacing`))))))
    (bind _returnvalue_2 (`KismetStringLibrary.GetSubstring` (`self.RandomCode`) _index))
    (switch `string` _returnvalue_2
      (:`A`
        (set `self.Color` (`self.Color_Green`)))
      (:`B`
        (set `self.Color` (`self.Color_Red`)))
      (:`C`
        (set `self.Color` (`self.Color_Blue`)))
      (:`D`
        (set `self.Color` (`self.Color_Yellow`))))
    (`MeshComponent.SetVectorParameterValueOnMaterials` _returnvalue "Color" (`self.Color`))
    (bind _returnvalue_3 (`AddComponent|NODE_AddBoxComponent-2` :`RelativeTransform` (`KismetMathLibrary.MakeTransform` (+ (`SceneComponent.RelativeLocation` _returnvalue) (0.0 0.0 20.0)))))
    (set `ActorComponent.ComponentTags` (`|MakeArray` (`KismetStringLibrary.Conv_StringToName` _returnvalue_2)) _returnvalue_3)
    (add `PrimitiveComponent.OnComponentBeginOverlap` _returnvalue_3 (`|CreateDelegate` :!event `Bp_Plaquepression_AutoGenFunc`))))

(event `self.ReceiveTick`
  (params (DeltaSeconds :type "Float (single-precision)"))
  (`KismetSystemLibrary.PrintString` (`self.Inputcode`) true true (struct :`G` 0.66 :`B` 1.0 :`A` 1.0) 0.0))

(fn `AddCode`
  (params (Add :type String))
  (bind _output_get (set `self.Start Index` (+ (`self.Start Index`) 1)))
  (if (== (`KismetStringLibrary.GetSubstring` (`self.CorrectCode`) _output_get) Add)
    (set `self.Inputcode` (`KismetStringLibrary.Concat_StrStr` (`self.Inputcode`) Add))
    (if (== (`KismetStringLibrary.Len` (`self.CorrectCode`)) (`KismetStringLibrary.Len` (`self.Inputcode`)))
      (if (== (`self.CorrectCode`) (`self.Inputcode`))
        (`KismetSystemLibrary.PrintString` "REUSSIT")
        (set `/Game/PapillonGame/Thomas_B/Blueprints/Bp_FinNiveau.PlaqueDone` true (`self.RefFinNiveau`))
        (else
          (set `self.Inputcode` "" :!label _label))))
    (else
      (set `self.Start Index` -1)
      (goto _label))))

(fn `Bp_Plaquepression_AutoGenFunc`
  (params (OverlappedComponent :type "PrimitiveComponent Object Reference") (OtherActor :type "Actor Object Reference") (OtherComp :type "PrimitiveComponent Object Reference") (OtherBodyIndex :type Integer) (bFromSweep :type Boolean) (SweepResult :type "HitResult Structure (by ref)"))
  (cast `/Game/PapillonGame/Thomas_B/ThirdPerson/Blueprints/BP_ThirdPersonCharacter` OtherActor)
  (`self.AddCode` (`KismetStringLibrary.Conv_NameToString` (`|GetArrayItem` (`ActorComponent.ComponentTags` OverlappedComponent))))
  (return))

(fn `UserConstructionScript`)