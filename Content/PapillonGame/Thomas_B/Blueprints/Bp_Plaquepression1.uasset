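; Pressure plate puzzle Blueprint, apparently meant for entering a code by stepping on plates, but unfinished.
; The construction script spawns a spaced row of plate meshes, each with a trigger box above it bound to an overlap handler.
; When the third-person character overlaps a box, its tag goes to AddCode, whose array write is incompletely wired.
; Tags are placeholder "None", and the code comparison with success or reset never runs.
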(event `self.ReceiveBeginPlay`)

(fn `AddCode`
  (params (Add :type String))
  (`KismetArrayLibrary.Array_Set` (`self.InputCode_0`)))

(fn `Bp_Plaquepression_AutoGenFunc`
  (params (OverlappedComponent :type "PrimitiveComponent Object Reference") (OtherActor :type "Actor Object Reference") (OtherComp :type "PrimitiveComponent Object Reference") (OtherBodyIndex :type Integer) (bFromSweep :type Boolean) (SweepResult :type "HitResult Structure (by ref)"))
  (cast `/Game/PapillonGame/Thomas_B/ThirdPerson/Blueprints/BP_ThirdPersonCharacter` OtherActor)
  (`self.AddCode` (`KismetStringLibrary.Conv_NameToString` (`|GetArrayItem` (`ActorComponent.ComponentTags` OverlappedComponent))))
  (`KismetSystemLibrary.PrintString` "Hello")
  (return))

(fn `UserConstructionScript`
  (for _index (range (`self.NumbersOfPlaque`))
    (bind _returnvalue (`AddComponent|NODE_AddStaticMeshComponent-1` :`RelativeTransform` (`KismetMathLibrary.MakeTransform` (`KismetMathLibrary.MakeVector` (* _index (`self.Spacing`))))))
    (bind _returnvalue_2 (`AddComponent|NODE_AddBoxComponent-1` :`RelativeTransform` (`KismetMathLibrary.MakeTransform` (+ (`SceneComponent.RelativeLocation` _returnvalue) (0.0 0.0 20.0)))))
    (set `ActorComponent.ComponentTags` (`|MakeArray` "None" :!type "Name") _returnvalue_2)
    (add `PrimitiveComponent.OnComponentBeginOverlap` _returnvalue_2 (`|CreateDelegate` :!event `Bp_Plaquepression_AutoGenFunc`))
    (`KismetArrayLibrary.Array_Add` (`self.InputCode_0`))))